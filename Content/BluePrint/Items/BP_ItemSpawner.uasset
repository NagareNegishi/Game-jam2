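; BP_ItemSpawner periodically spawns items at random positions within a configurable area, up to a population cap.
; A looping timer started on BeginPlay fires every Interval and counts existing BP_ZZZ actors in the level.
; Below MaxItem, it spawns one ItemType actor at random X and Y within the bounds and a fixed low Z.
; The count uses the hardcoded BP_ZZZ class rather than ItemType.
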(event Custom|spawnitems
  (bind _outactors (Actor|GetAllActorsOfClass "/Game/BluePrint/Items/BP_ZZZ.BP_ZZZ_C"))
  (if (< (Utilities|Array|Length _outactors) (Variables|Default|GetMax%20Item))
    (Game|SpawnActorfromClass (Variables|Default|GetItemType) (Math|Conversions|ToTransform(Vector) (Math|Vector|MakeVector (Math|Random|RandomFloatinRange (Variables|Default|GetMinX) (Variables|Default|GetMaxX)) (Math|Random|RandomFloatinRange (Variables|Default|GetMinY) (Variables|Default|GetMaxY)) 1e+01)) "Undefined" "MultiplyWithRoot" 0 3e+02 "0.000000,0.000000,0.000000" 0)))

(event EventBeginPlay
  (Utilities|Time|SetTimerbyEvent (delegate Custom|spawnitems) (Variables|Default|GetInterval) true))

(fn ConstructionScript)