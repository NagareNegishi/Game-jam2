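; BP_Taka is an enemy Blueprint that periodically picks an actor of a target class to follow.
; A looping timer started on BeginPlay scans all such actors and stores one in Follow.
; Despite the Closest variable name, the greater-than comparison selects the farthest actor.
; Three movement approaches (movement input, AIMoveTo, MoveComponentTo) are disconnected, so this graph never moves it toward Follow.
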(event Custom|searchitem
  (Variables|Default|SetClosest 0.0)
  (bind _outactors (Actor|GetAllActorsOfClass (Variables|Default|GetTarget)))
  (if (not (Utilities|Array|IsEmpty _outactors))
    (for _array_element _outactors
      (if (> (Math|Vector|Distance(Vector) (Transformation|GetActorLocation _array_element) (Transformation|GetActorLocation)) (Variables|Default|Getclosest))
        (Variables|Default|Setclosest (Math|Vector|Distance(Vector) (Transformation|GetActorLocation _array_element) (Transformation|GetActorLocation)))
        (Variables|Default|SetFollow _array_element)))))

(event EventBeginPlay
  (Utilities|Time|SetTimerbyEvent (delegate Custom|searchitem) 2.0 true))

(event Collision|EventActorBeginOverlap
  (params (OtherActor :type Actor%20Object%20Reference)))

(event EventTick
  (params (DeltaSeconds :type Float%20%28single-precision%29)))

(fn ConstructionScript)