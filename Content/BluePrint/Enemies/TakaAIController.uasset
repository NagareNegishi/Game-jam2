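; TakaAIController is an enemy AI controller that periodically sends its pawn after an actor of the TargetItem class.
; A looping timer started on BeginPlay scans all such actors, compares their distances to the pawn and moves it to the selected one.
; Although the variable is named Closest, it starts at zero and uses a greater-than test, so the farthest item wins.
; Debug prints trace each search.
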(event Custom|searchitem
  (Variables|Default|Setclosest 0.0)
  (Development|PrintString "before loop")
  (bind _outactors (Actor|GetAllActorsOfClass (Variables|Default|GetTargetItem)))
  (if (Utilities|Array|IsEmpty _outactors)
    (Development|PrintString "empty")
    (else
      (for _array_element _outactors
        (if (> (Math|Vector|Distance(Vector) (Transformation|GetActorLocation _array_element) (Transformation|GetActorLocation (Pawn|GetControlledPawn))) (Variables|Default|Getclosest))
          (Variables|Default|Setclosest (Math|Vector|Distance(Vector) (Transformation|GetActorLocation _array_element) (Transformation|GetActorLocation (Pawn|GetControlledPawn))))
          (Variables|Default|SetfollowIt _array_element)
          (else
            (Development|PrintString "im not"))))
      (AI|Navigation|MovetoActor (Variables|Default|GetfollowIt) 5e+01 true true true 0)
      (Development|PrintString (Utilities|GetDisplayName (Variables|Default|GetfollowIt)))
      (Development|PrintString (Utilities|String|ToString(Vector) (Transformation|GetActorLocation (Variables|Default|GetfollowIt))))
      (Development|PrintString "but im at")
      (Development|PrintString (Utilities|String|ToString(Vector) (Transformation|GetActorLocation (Pawn|GetControlledPawn)))))))

(event EventBeginPlay
  (Utilities|Time|SetTimerbyEvent (delegate Custom|searchitem) (Variables|Default|GetserchInterval) true)
  (Development|PrintString "first"))

(fn ConstructionScript)