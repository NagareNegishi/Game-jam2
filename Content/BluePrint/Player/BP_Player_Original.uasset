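; Player character with top-down style movement that fires bullets from a ring of summoned shooters, with background music and walk sounds.
; Space spawns the BP_Player_Shooter ring once, attached to a spring arm that spins every Tick.
; Debug-style keys tune fire interval, bullet speed and spin, stop firing, or damage the HealthComponent.
; Movement input picks one of four facings for the Nasu1 component; the 180-degree sweep rotation is unused.
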(event OnDamageTaken(HealthComponent)
  (Development|PrintString (Utilities|String|ToString(Float) (Variables|/Game/BluePrint/ActorComponents/HealthComponent.HealthComponent_C|GetHealth (Variables|Default|GetHealthComponent)))))

(event Input|EnhancedActionEvents|EnhancedInputActionMove
  (params (ActionValue :type Vector%202D%20Structure) (ElapsedSeconds :type Float%20%28double-precision%29) (TriggeredSeconds :type Float%20%28double-precision%29) (InputAction :type Input%20Action%20Object%20Reference :default "/Game/Input/Move.Move"))
  ;[1 1 1] Move and Sound
  (if (Variables|Default|GetCanMove)
    (Pawn|Input|AddMovementInput "1.000000,0.000000,0.000000" (.x ActionValue) false)
    (Pawn|Input|AddMovementInput "0.000000,1.000000,0.000000" (.y ActionValue) false)
    (if (Variables|Default|GetWalkingSound)
      (if (Utilities|IsValid (stale _returnvalue))
        _
        (else
          (Variables|Default|SetWalkingSound false)))
      (else
        (bind _returnvalue (Audio|SpawnSoundatLocation (Variables|Default|GetWalkSound) "0, 0, 0" "0, 0, 0" 1.0 1.0 0.0 0 0))
        (Variables|Default|SetWalkingSound true)))
    (CallFunction|CheckDirection (.x ActionValue) (.y ActionValue))))

(event EventBeginPlay
  ;[1 1 1] controller setting
  (bind _asplayer_controller (Utilities|Casting|CastToPlayerController (Pawn|GetController)))
  (Utilities|IsValid (PlayerController|LocalPlayerSubsystems|GetEnhancedInputLocalPlayerSubsystem _asplayer_controller)
    (:Is%20Valid
      (Input|AddMappingContext (PlayerController|LocalPlayerSubsystems|GetEnhancedInputLocalPlayerSubsystem _asplayer_controller) "/Game/Input/Control.Control" 0 "(bIgnoreAllPressedKeysUntilRelease=True,bForceImmediately=False,bNotifyUserSettings=False)")
      (Audio|SpawnSound2D "/Game/Music/Traditional_Japanese_dream_with_happy_ghost__8e59be1234b346809544690380ce5462_.Traditional_Japanese_dream_with_happy_ghost__8e59be1234b346809544690380ce5462_" 1.0 1.0 0.0 0))))

(event Collision|EventActorBeginOverlap
  (params (OtherActor :type Actor%20Object%20Reference)))

(event EventTick
  (params (DeltaSeconds :type Float%20%28single-precision%29))
  (Utilities|FlowControl|Sequence
    (:then_0
      (CallFunction|UpdateAnimation))
    (:then_1
      ;[1 1 1] rotate version
      (Transformation|AddLocalRotation (Variables|Default|GetSpringArm_Shooter) (Math|Rotator|MakeRotator 0.0 0.0 (Variables|ShooterSetting|GetShooterRotateSpeed)) false false))))

(event Input|KeyboardEvents|X
  (params (Key :type Key%20Structure))
  (:Pressed
    (Default|TakeDamege (Variables|Default|GetHealthComponent) 2e+01)))

(event Input|KeyboardEvents|SpaceBar
  (params (Key :type Key%20Structure))
  ;[1 1 1] Summon Shooter
  (:Pressed
    (Utilities|FlowControl|DoOnce false
      (:Completed
        (CallFunction|SummonShooter (Transformation|GetActorLocation) (Variables|ShooterSetting|GetShooterRadius) (Variables|ShooterSetting|GetShooterNumber))))))

(event Input|KeyboardEvents|Z
  (params (Key :type Key%20Structure))
  ;[1 1 1] CommentShoot Frequency
  (:Pressed
    (bind _output_get (Variables|ShooterSetting|SetShooterFrequency (- (Variables|ShooterSetting|GetShooterFrequency) 0.1)))
    (if (<= _output_get 0.1)
      (Variables|ShooterSetting|SetShooterFrequency 0.1))
    (CallFunction|UpdateShooterFrequency (Variables|ShooterSetting|GetShooterFrequency))))

(event Input|KeyboardEvents|V
  (params (Key :type Key%20Structure))
  ;[1 1 1] Shoot Speed
  (:Pressed
    (bind _output_get (Variables|ShooterSetting|SetBulletSpeed (+ (Variables|ShooterSetting|GetBulletSpeed) 1e+02)))
    (if (> _output_get (Variables|ShooterSetting|GetBulletMaxSpeed))
      (Variables|ShooterSetting|SetBulletSpeed (Variables|ShooterSetting|GetBulletMaxSpeed)))
    (CallFunction|UpdateShooterSpeed (Variables|ShooterSetting|GetBulletSpeed))))

(event Input|KeyboardEvents|C
  (params (Key :type Key%20Structure))
  ;[1 1 1] may not need it
  (:Pressed
    (bind _output_get (Variables|ShooterSetting|SetShooterRotateSpeed (+ (Variables|ShooterSetting|GetShooterRotateSpeed) 3.0)))
    (CallFunction|UpdateRotationSpeed _output_get)))

(event Input|KeyboardEvents|C
  (params (Key :type Key%20Structure))
  ;[1 1 1] Stop Shooting
  (:Pressed
    (CallFunction|StopShooting)))

(fn ConstructionScript)

(fn SummonShooter
  (params (Center :type Vector) (Radius :type Float%20%28double-precision%29) (ObjectNumber :type Integer))
  (Variables|ShooterSetting|SetShooterAngle (/ (* (Math|Trig|GetPI) 2.0) ObjectNumber))
  (for _index (range 0 (- ObjectNumber 1))
    (bind _returnvalue (Game|SpawnActorfromClass :Class "/Game/BluePrint/Player/BP_Player_Shooter.BP_Player_Shooter_C" :SpawnTransform (Math|Transform|MakeTransform (Math|Vector|MakeVector (+ (.x Center) (* Radius (Math|Trig|Cos(Radians) (* (Variables|ShooterSetting|GetShooterAngle) _index)))) (+ (.y Center) (* Radius (Math|Trig|Sin(Radians) (* (Variables|ShooterSetting|GetShooterAngle) _index)))) (.z Center)) "0, 0, 0" "1.000000,1.000000,1.000000") :CollisionHandlingOverride "Undefined" :TransformScaleMethod "MultiplyWithRoot" :ProjectileType "/Game/BluePrint/Projectiles/BP_Projectile_Bullet.BP_Projectile_Bullet_C" :Frequency (Variables|ShooterSetting|GetShooterFrequency) :BulletSpeed (Variables|ShooterSetting|GetBulletSpeed) :Instigator 0))
    (Utilities|Array|Add (Variables|ShooterSetting|GetShooters) _returnvalue)
    (Transformation|AttachComponentToComponent _returnvalue (Variables|Default|GetSpringArm_Shooter) "None" "KeepWorld" "KeepWorld" "KeepWorld" true)))

(fn UpdateShooterFrequency
  (params (Frequency :type Float%20%28double-precision%29))
  (for _array_element (Variables|ShooterSetting|GetShooters)
    (Default|UpdateFrequency _array_element (Variables|ShooterSetting|GetShooterFrequency))))

(fn UpdateShooterSpeed
  (params (Speed :type Float%20%28double-precision%29))
  (for _array_element (Variables|ShooterSetting|GetShooters)
    (Default|UpdateBulletSpeed _array_element (Variables|ShooterSetting|GetBulletSpeed))))

(fn UpdateProjectileType
  (params (Type :type BP%20Projectile%20Base%20Class%20Reference))
  (for _array_element (Variables|ShooterSetting|GetShooters)
    (Default|UpdateProjectileType _array_element (Variables|ShooterSetting|GetProjectileType))))

(fn UpdateRotationSpeed
  (params (RotateSpeed :type Float%20%28double-precision%29))
  (Variables|ShooterSetting|SetShooterRotateSpeed RotateSpeed))

(fn 180Rotation
  (params (delta :type Float%20%28double-precision%29))
  (if (Variables|Shooter180rotation|GetMovingRight)
    (if (>= (+ (Variables|ShooterSetting|GetShooterRotateSpeed) (Variables|Shooter180rotation|GetCurrentAngle)) 1.8e+02)
      (Variables|Shooter180rotation|SetMovingRight false)
      (else
        (bind _output_get (Variables|Shooter180rotation|SetCurrentAngle (+ (Variables|ShooterSetting|GetShooterRotateSpeed) (Variables|Shooter180rotation|GetCurrentAngle))))
        (Transformation|SetRelativeRotation (Variables|Default|GetSpringArm_Shooter) (Math|Rotator|MakeRotator 0.0 0.0 _output_get) false false)))
    (elif (<= (+ (* (Variables|ShooterSetting|GetShooterRotateSpeed) -1.0) (Variables|Shooter180rotation|GetCurrentAngle)) 0.0)
      (Variables|Shooter180rotation|SetMovingRight true)
      (else
        (bind _output_get_2 (Variables|Shooter180rotation|SetCurrentAngle (+ (* (Variables|ShooterSetting|GetShooterRotateSpeed) -1.0) (Variables|Shooter180rotation|GetCurrentAngle))))
        (Transformation|SetRelativeRotation (Variables|Default|GetSpringArm_Shooter) (Math|Rotator|MakeRotator 0.0 0.0 _output_get_2) false false)))))

(fn CheckDirection
  (params (X :type Float%20%28double-precision%29) (Y :type Float%20%28double-precision%29))
  (if (> (Math|Float|Absolute(Float) X) (Math|Float|Absolute(Float) Y))
    (if (> X 0.0)
      (Variables|Default|SetDir "NewEnumerator0")
      (else
        (Variables|Default|SetDir "NewEnumerator1")))
    (elif (> Y 0.0)
      (Variables|Default|SetDir "NewEnumerator2")
      (else
        (Variables|Default|SetDir "NewEnumerator3")))))

(fn StopShooting
  (for _array_element (Variables|ShooterSetting|GetShooters)
    (Default|UpdateFrequency _array_element 0.0)))

(fn UpdateAnimation
  (switch Utilities|FlowControl|Switch|SwitchonPlayerDir (Variables|Default|GetDir)
    (:NewEnumerator0
      (Transformation|SetRelativeRotation (Variables|Default|Getnasu1) "0.000000,0.000000,270.000000" false false))
    (:NewEnumerator1
      (Transformation|SetRelativeRotation (Variables|Default|Getnasu1) "180.000000,0.000000,90.000000" false false))
    (:NewEnumerator2
      (Transformation|SetRelativeRotation (Variables|Default|Getnasu1) "0.000000,90.000000,270.000000" false false))
    (:NewEnumerator3
      (Transformation|SetRelativeRotation (Variables|Default|Getnasu1) "180.000000,90.000000,270.000000" false false))))